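; Interactable button that dips when used and triggers actions on target objects implementing BI_ButtonObject, printing a warning if none qualify.
; BeginPlay binds ButtonPressed to an action that messages the BeginPlay loop's current element, not each target separately.
; One timeline, flipped by IsPressed, lowers and raises the actor around a hold, blocking re-presses until finished.
; ButtonPressed fires after a construction-computed delay of timeline length plus hold time.
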(event `self.ReceiveBeginPlay`
  (for _array_element (`self.TargetObjects`)
    (if (`KismetSystemLibrary.DoesImplementInterface` _array_element "/Game/_Presentation/Level1/Blueprints/Interfaces/BI_ButtonObject.BI_ButtonObject_C")
      (add `self.ButtonPressed` (delegate `DoAssignedAction`))
      (set `self.ControllesObjects` true)))
  (if (not (`self.ControllesObjects`))
    (`KismetSystemLibrary.PrintString` (`KismetStringLibrary.Concat_StrStr` (`KismetSystemLibrary.GetDisplayName` self) " will do nothing if pressed!"))))

(event `DoAssignedAction`
  (message `/Game/_Presentation/Level1/Blueprints/Interfaces/BI_ButtonObject.DoAction` (stale `self.ReceiveBeginPlay` _array_element)))

(event `/Game/_Presentation/Level1/Blueprints/Interfaces/BI_Interactable.OnInteract`
  (if (`self.IsAvailable`)
    (`self.PressButton`)
    (`KismetSystemLibrary.Delay` (`self.ButtonHandlerDelay`))
    (`self.ButtonPressed`)))

(event `PressButton`
  (set `self.IsAvailable` false)
  (set `self.IsPressed` false)
  (bind (_direction _buttondown _buttonup) (`Timeline|ButtonAnimationTimeline` :!via `PlayFromStart` :!label _label)
    (:`Update`
      (if (`self.IsPressed`)
        (`self.K2_SetActorLocation` (`KismetMathLibrary.VLerp` (`self.EndPoint`) (`self.StartPoint`) _buttonup))
        (else
          (`self.K2_SetActorLocation` (`KismetMathLibrary.VLerp` (`self.StartPoint`) (`self.EndPoint`) _buttondown)))))
    (:`Finished`
      (set `self.IsPressed` (not (`self.IsPressed`)))
      (if (`self.IsPressed`)
        (`KismetSystemLibrary.Delay` (`self.PressedDuration`))
        (goto _label :!via `PlayFromStart`)
        (else
          (set `self.IsAvailable` true))))))

(event `/Game/_Presentation/Level1/Blueprints/Interfaces/BI_Aimable.OnAimed`
  (`KismetSystemLibrary.PrintString` "Button aimed"))

(event `/Game/_Presentation/Level1/Blueprints/Interfaces/BI_Aimable.OnAimedEnd`
  (`KismetSystemLibrary.PrintString` "Button unaimed"))

(fn `CheckAvailability`
  (returns (IsAvailable :type Boolean))
  (return (`self.IsAvailable`)))

(fn `SetStartAndEnd`
  (bind _output_get (set `self.StartPoint` (`self.K2_GetActorLocation`)))
  (set `self.EndPoint` (- _output_get (0.0 0.0 3.0))))

(fn `UserConstructionScript`
  (set `self.ButtonHandlerDelay` (+ (`TimelineComponent.GetTimelineLength` (`self.ButtonAnimationTimeline`)) (`self.PressedDuration`)))
  (`self.SetStartAndEnd`))