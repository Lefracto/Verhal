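; BP_MovingButton is a movable Blueprint in Level1 that carries a button which only becomes usable after it finishes moving.
; BeginPlay disables BPButton, and the end-of-moving event later calls its SetStartAndEnd and makes it available.
; DoSomething starts the inherited Move, while construction turns off collision triggering and CheckAvailability always returns false.
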(event `self.ReceiveBeginPlay`
  (`parent.ReceiveBeginPlay`)
  (set `/Game/_Presentation/Level1/Blueprints/Interactable/BP_Button.IsAvailable` false (`self.BP_Button`))
  (add `self.EndOfMoving` (delegate `MakeButtonAvailable`)))

(event `MakeButtonAvailable`
  (bind _bp_button (`self.BP_Button`))
  (`/Game/_Presentation/Level1/Blueprints/Interactable/BP_Button.SetStartAndEnd` _bp_button)
  (set `/Game/_Presentation/Level1/Blueprints/Interactable/BP_Button.IsAvailable` true _bp_button))

(event `/Game/_Presentation/Level1/Blueprints/Interfaces/BI_AfterDeathObject.DoSomething`
  (`self.Move`))

(fn `CheckAvailability`
  (returns (IsAvailable :type Boolean))
  (return false))

(fn `UserConstructionScript`
  (`parent.UserConstructionScript`)
  (set `self.TriggerOnCollision` false))