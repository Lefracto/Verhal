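; BP_MovingWall is a movable wall that calls Move when it receives an OnInteract event.
; CheckAvailability reports it as unavailable once Triggered is set.
; Before that, a normal wall is always available, while one flagged IsSecret is available only when the player pawn's IsDefaultColorMessage returns false.
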(event `/Game/_Presentation/Level1/Blueprints/Interfaces/BI_Interactable.OnInteract`
  (`self.Move`))

(fn `CheckAvailability`
  (returns (IsAvailable :type Boolean))
  (if (`self.IsSecret`)
    (if (not (`self.Triggered`))
      (bind _newparam (message `/Game/_Presentation/Level1/Blueprints/Interfaces/WallColorManager.IsDefaultColor` (`GameplayStatics.GetPlayerPawn` 0)))
      (return (not _newparam))
      (else
        _))
    (elif (`self.Triggered`)
      _
      (else
        (return true))))
  (return false))

(fn `UserConstructionScript`
  (`parent.UserConstructionScript`))