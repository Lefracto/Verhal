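; Level actor that slides between its start location and an EndPoint, triggered by DoAction or optionally by the player pawn overlapping its collision.
; Move waits for MoveDelay, then a timeline with Speed as play rate drives a swept lerp between the two points.
; When finished, it swaps the endpoints so the next move returns, then calls EndOfMoving.
; The construction script applies the configurable Material to the mesh.
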(event `self.ReceiveBeginPlay`
  (`TimelineComponent.SetPlayRate` (`self.SlideTimeline`) (`self.Speed`))
  (set `self.StartPoint` (`self.K2_GetActorLocation`)))

(event `Move`
  (set `self.Triggered` (not (`self.Triggered`)))
  (`KismetSystemLibrary.Delay` (`self.MoveDelay`))
  (bind (_direction _slidecurve) (`Timeline|SlideTimeline` :!via `PlayFromStart`)
    (:`Update`
      (`self.K2_SetActorLocation` (`KismetMathLibrary.VLerp` (`self.StartPoint`) (`self.EndPoint`) _slidecurve) true))
    (:`Finished`
      (set `self.EndPoint` (`self.StartPoint`))
      (set `self.StartPoint` (`self.K2_GetActorLocation`))
      (`self.EndOfMoving`))))

(event `self.Collision.OnComponentBeginOverlap`
  (params (OverlappedComponent :type "PrimitiveComponent Object Reference") (OtherActor :type "Actor Object Reference") (OtherComp :type "PrimitiveComponent Object Reference") (OtherBodyIndex :type Integer) (bFromSweep :type Boolean) (SweepResult :type "HitResult Structure (by ref)"))
  (if (and (`self.TriggerOnCollision`) (== OtherActor (`GameplayStatics.GetPlayerPawn` 0)))
    (`self.Move`)))

(event `/Game/_Presentation/Level1/Blueprints/Interfaces/BI_ButtonObject.DoAction`
  (`self.Move`))

(fn `UserConstructionScript`
  (`PrimitiveComponent.SetMaterial` (`self.Mesh`) 0 (`self.Material`)))