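; BP_HidingInteractable is an always-available interactable that applies its configured material at construction and shows an outline overlay while aimed at.
; Interacting fires CallLastInteraction, then KillChildren.
; When ShouldCallSomeone is set, it binds to the LastInteraction event at BeginPlay to trigger DoSomething on SomeObject, provided that object implements BI_AfterDeathObject.
; Aim changes also print debug strings.
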(event `self.ReceiveBeginPlay`
  (`parent.ReceiveBeginPlay`)
  (if (`self.ShouldCallSomeone`)
    (add `self.LastInteraction` (delegate `CallSomeone`))))

(event `CallSomeone`
  (if (`KismetSystemLibrary.DoesImplementInterface` (`self.SomeObject`) "/Game/_Presentation/Level1/Blueprints/Interfaces/BI_AfterDeathObject.BI_AfterDeathObject_C")
    (message `/Game/_Presentation/Level1/Blueprints/Interfaces/BI_AfterDeathObject.DoSomething` (`self.SomeObject`))))

(event `/Game/_Presentation/Level1/Blueprints/Interfaces/BI_Interactable.OnInteract`
  (`self.LastInteraction`)
  (`self.KillChildren`))

(event `/Game/_Presentation/Level1/Blueprints/Interfaces/BI_Aimable.OnAimed`
  (`KismetSystemLibrary.PrintString` "Aimed")
  (`MeshComponent.SetOverlayMaterial` (`self.Mesh`) (`self.OutlineMaterial`)))

(event `/Game/_Presentation/Level1/Blueprints/Interfaces/BI_Aimable.OnAimedEnd`
  (`KismetSystemLibrary.PrintString` "Unaimed")
  (`MeshComponent.SetOverlayMaterial` (`self.Mesh`) null))

(fn `CheckAvailability`
  (returns (IsAvailable :type Boolean))
  (return true))

(fn `UserConstructionScript`
  (`parent.UserConstructionScript`)
  (`PrimitiveComponent.SetMaterial` (`self.Mesh`) 0 (`self.Material`)))