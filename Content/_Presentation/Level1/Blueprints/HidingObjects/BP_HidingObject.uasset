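; BP_HidingObject is a Level 1 presentation actor that can remove either itself or selected parts of itself.
; On BeginPlay, unless ShouldIKillMyself is set, it caches the direct children of DefaultSceneRoot tagged "Killable".
; The KillChildren event destroys the whole actor when that flag is set, and otherwise destroys only the cached components.
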(event `self.ReceiveBeginPlay`
  (if (not (`self.Should_I_Kill_Myself`))
    (`KismetArrayLibrary.Array_Clear` (`self.KillableChildren`))
    (for _array_element (`SceneComponent.GetChildrenComponents` (`self.DefaultSceneRoot`) false)
      (`/Engine/EditorBlueprintResources/StandardMacros.IsValid` _array_element
        (:`Is Valid`
          (if (`ActorComponent.ComponentHasTag` _array_element "Killable")
            (`KismetArrayLibrary.Array_Add` (`self.KillableChildren`) _array_element)))))))

(event `KillChildren`
  (if (`self.Should_I_Kill_Myself`)
    (`self.K2_DestroyActor`)
    (else
      (for _array_element (`self.KillableChildren`)
        (`ActorComponent.K2_DestroyComponent` _array_element)))))

(fn `UserConstructionScript`)