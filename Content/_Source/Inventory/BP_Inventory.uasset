(event `Key|E`
  (params (Key :type "Key Structure"))
  (bind _firstpersoncamera (`/Game/FirstPerson/Blueprints/BP_FirstPersonCharacter.FirstPersonCamera` (`self.FirstPersonCamera`)))
  (bind _returnvalue (`SceneComponent.K2_GetComponentLocation` _firstpersoncamera))
  (:`Pressed`
    (bind _outhit (`KismetSystemLibrary.LineTraceSingle` _returnvalue (+ _returnvalue (* (`KismetMathLibrary.GetForwardVector` (`SceneComponent.K2_GetComponentRotation` _firstpersoncamera)) 500)) "TraceTypeQuery1"))
    (bind _asbp_item (cast `/Game/_Source/Inventory/BP_Item` (`.HitActor` (`GameplayStatics.BreakHitResult` _outhit))))
    (for (_array_element _array_index) (`self.Items`)
      (`/Engine/EditorBlueprintResources/StandardMacros.IsValid` _asbp_item
        (:`Is Valid`
          (bind (_name _stackable _count) (break `/Game/_Source/Inventory/S_ItemStruct` _array_element))
          (bind _item (`/Game/_Source/Inventory/BP_Item.Item` _asbp_item))
          (bind (_name_2 _stackable_2 _count_2) (break `/Game/_Source/Inventory/S_ItemStruct` _item))
          (bind _returnvalue_2 (+ _count _count_2))
          (if (and (`KismetTextLibrary.EqualEqual_TextText` _name _name_2) _stackable_2 (<= _returnvalue_2 64))
            (bind (_name_3 _stackable_3 _count_3 _icon _mesh _description) (break `/Game/_Source/Inventory/S_ItemStruct` _item))
            (`KismetArrayLibrary.Array_Set` (`self.Items`) _array_index (make `/Game/_Source/Inventory/S_ItemStruct` _name_3 _stackable_3 _returnvalue_2 _icon _mesh _description))
            (`/Game/_Source/Inventory/WB_Inventory.LoadInventory` (`self.InventoryWidget`) self :!label _label)
            (`Actor.K2_DestroyActor` _asbp_item)
            (elif (== _count 0)
              (`KismetArrayLibrary.Array_Set` (`self.Items`) _array_index (`/Game/_Source/Inventory/BP_Item.Item` _asbp_item))
              (goto _label))))))))

(event `self.ReceiveBeginPlay`
  (bind _returnvalue (`|CreateWidget` "/Game/_Source/Inventory/WB_Inventory.WB_Inventory_C"))
  (set `self.InventoryWidget` _returnvalue)
  (`KismetArrayLibrary.Array_Resize` (`self.Items`) 10)
  (`/Game/_Source/Inventory/WB_Inventory.LoadInventory` (`self.InventoryWidget`) self)
  (bind _asbp_first_person_character (cast `/Game/FirstPerson/Blueprints/BP_FirstPersonCharacter` (`GameplayStatics.GetPlayerCharacter` 0)))
  (set `self.FirstPersonCamera` _asbp_first_person_character))

(event `Key|I`
  (params (Key :type "Key Structure"))
  (bind _returnvalue (`GameplayStatics.GetPlayerController` 0))
  (bind _returnvalue_2 (`GameplayStatics.GetPlayerController` 0))
  (bind _inventorywidget (`self.InventoryWidget`))
  (:`Pressed`
    (`self.ClearOptionsMenu`)
    (`/Game/_Source/Inventory/WB_Inventory.ClearDescription` (`self.InventoryWidget`))
    (if (`Widget.IsVisible` (`self.InventoryWidget`))
      (`Widget.RemoveFromParent` _inventorywidget)
      (set `PlayerController.bShowMouseCursor` false _returnvalue)
      (`WidgetBlueprintLibrary.SetInputMode_GameOnly` _returnvalue)
      (else
        (set `PlayerController.bShowMouseCursor` true _returnvalue_2)
        (`WidgetBlueprintLibrary.SetInputMode_GameAndUIEx` _returnvalue_2 null)
        (`UserWidget.AddToViewport` _inventorywidget 0)))))

(fn `ClearOptionsMenu`
  (`/Game/_Source/Inventory/WB_Inventory.ClearOptionsMenu` (`self.InventoryWidget`)))

(fn `SelectItem`
  (params (index :type Integer)))