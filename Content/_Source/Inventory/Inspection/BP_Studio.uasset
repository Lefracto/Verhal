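; BP_Studio is an inventory inspection actor that displays a chosen item's static mesh for the player to examine.
; Inspect sets the mesh, shows WB_Inspection, disables the player's input and enables its own.
; CalledMouseX and CalledMouseY apply yaw and pitch to the mesh through CombineRotators while CanRotate is true.
; Exit restores player input, removes the widget and destroys the actor.
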(event `/Game/_Source/Inventory/Inspection/InspectableItem.Inspect`
  (params (Player :type "/Game/FirstPerson/Blueprints/BP_FirstPersonCharacter Object Reference") (`Item to focus` :type "StaticMesh Object Reference"))
  (set `self.Player` Player)
  (`StaticMeshComponent.SetStaticMesh` (`self.Item`) `Item to focus`)
  (bind _returnvalue (`|CreateWidget` "/Game/_Source/Inventory/Inspection/WB_Inspection.WB_Inspection_C"))
  (set `self.InspectWidget` _returnvalue)
  (`UserWidget.AddToViewport` _returnvalue 0)
  (`self.DisableInput` (`self.Player`) (`GameplayStatics.GetPlayerController` 0))
  (`self.EnableInput` null))

(event `Key|LeftMouseButton`
  (params (Key :type "Key Structure")))

(event `self.ReceiveBeginPlay`)

(event `/Game/_Source/Inventory/Inspection/InspectableItem.Interact Items`)

(fn `CalledMouseX`
  (params (Axis :type "Float (double-precision)"))
  (if (`self.CanRotate`)
    (`SceneComponent.K2_SetWorldRotation` (`self.Item`) (`KismetMathLibrary.ComposeRotators` (`SceneComponent.K2_GetComponentRotation` (`self.Item`)) (`KismetMathLibrary.MakeRotator` 0.0 0.0 (* Axis -5.0))) false false)))

(fn `CalledMouseY`
  (params (Axis :type "Float (double-precision)"))
  (if (`self.CanRotate`)
    (`SceneComponent.K2_SetWorldRotation` (`self.Item`) (`KismetMathLibrary.ComposeRotators` (`SceneComponent.K2_GetComponentRotation` (`self.Item`)) (`KismetMathLibrary.MakeRotator` 0.0 (* Axis -5.0))) false false)))

(fn `Exit`
  (`self.EnableInput` (`self.Player`) (`GameplayStatics.GetPlayerController` 0))
  (`Widget.RemoveFromParent` (`self.InspectWidget`))
  (`self.K2_DestroyActor` self))

(fn `UserConstructionScript`)