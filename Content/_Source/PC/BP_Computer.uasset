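; BP_Computer is an in-world computer that switches the player's view to its own camera when the first-person character enters its Box.
; The overlap registers it as the character's CurrentInside, sets ShouldExit, caches the player camera and blends the view over.
; Leaving a separate Cube component clears ShouldExit without changing the view.
; The Exit event and near-duplicate ExitMode function, which adds a debug print, blend back to the player.
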(event `self.Box.OnComponentBeginOverlap`
  (params (OverlappedComponent :type "PrimitiveComponent Object Reference") (OtherActor :type "Actor Object Reference") (OtherComp :type "PrimitiveComponent Object Reference") (OtherBodyIndex :type Integer) (bFromSweep :type Boolean) (SweepResult :type "HitResult Structure (by ref)"))
  (bind _asbp_first_person_character (cast `/Game/FirstPerson/Blueprints/BP_FirstPersonCharacter` OtherActor))
  (set `/Game/FirstPerson/Blueprints/BP_FirstPersonCharacter.CurrentInside` self _asbp_first_person_character)
  (set `/Game/FirstPerson/Blueprints/BP_FirstPersonCharacter.ShouldExit` true _asbp_first_person_character)
  (set `self.PlayerCamera` (`/Game/FirstPerson/Blueprints/BP_FirstPersonCharacter.FirstPersonCamera` _asbp_first_person_character))
  (`PlayerController.SetViewTargetWithBlend` (`GameplayStatics.GetPlayerController` 0) (`ActorComponent.GetOwner` (`self.PcCamera`)) 1.0 "VTBlend_Linear" 0.0 false))

(event `Exit`
  (`/Engine/EditorBlueprintResources/StandardMacros.IsValid` (`self.PlayerCamera`)
    (:`Is Valid`
      (`PlayerController.SetViewTargetWithBlend` (`GameplayStatics.GetPlayerController` 0) (`ActorComponent.GetOwner` (`self.PlayerCamera`)) 1.0 "VTBlend_Linear" 0.0 false))))

(event `self.Cube.OnComponentEndOverlap`
  (params (OverlappedComponent :type "PrimitiveComponent Object Reference") (OtherActor :type "Actor Object Reference") (OtherComp :type "PrimitiveComponent Object Reference") (OtherBodyIndex :type Integer))
  (bind _asbp_first_person_character (cast `/Game/FirstPerson/Blueprints/BP_FirstPersonCharacter` OtherActor))
  (set `/Game/FirstPerson/Blueprints/BP_FirstPersonCharacter.ShouldExit` false _asbp_first_person_character))

(fn `ExitMode`
  (`/Engine/EditorBlueprintResources/StandardMacros.IsValid` (`self.PlayerCamera`)
    (:`Is Valid`
      (`KismetSystemLibrary.PrintString` "2")
      (`PlayerController.SetViewTargetWithBlend` (`GameplayStatics.GetPlayerController` 0) (`ActorComponent.GetOwner` (`self.PlayerCamera`)) 1.0 "VTBlend_Linear" 0.0 false))))

(fn `UserConstructionScript`)