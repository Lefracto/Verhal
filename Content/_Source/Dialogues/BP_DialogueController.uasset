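; Dialogue controller that plays branching conversations from the CDT_Dialogues data table through subtitle and reply widgets created on BeginPlay.
; StartDialogue looks up rows from a trigger name in a fixed six-pass loop containing Delays, typing each phrase in a speaker-specific color.
; Speaker 0 lines then show next-row texts as replies in UI-only input and index NextLines by ReplyID; speaker 1 lines take the first next line.
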(event `self.ReceiveBeginPlay`
  (bind _returnvalue (`|CreateWidget` "/Game/_Source/Dialogues/WB_Dialogue.WB_Dialogue_C" (`GameplayStatics.GetPlayerController` 0)))
  (bind _output_get (set `self.DialogueWidget` _returnvalue))
  (`UserWidget.AddToViewport` _output_get 0)
  (bind _returnvalue_2 (`|CreateWidget` "/Game/_Source/Dialogues/WB_DynamicSubtitles.WB_DynamicSubtitles_C" (`GameplayStatics.GetPlayerController` 0) "Preview"))
  (bind _output_get_2 (set `self.SubtitlesWidget` _returnvalue_2))
  (`UserWidget.AddToViewport` _output_get_2 0))

(event `StartDialogue`
  (params (DialogueTrigger :type Name))
  (set `self.CurrentLIneName` DialogueTrigger)
  (for _ (range 6)
    (bind _returnvalue (`|GetDataTableRow` "/Game/_Source/Dialogues/CDT_Dialogues.CDT_Dialogues" (`self.CurrentLIneName`))
      (:`then`
        (bind (_text _speakerid _previousline _nextline) (break `/Game/_Source/Dialogues/ST_DialogueLine` _returnvalue))
        (set `self.CurrentPhrase` _text)
        (set `self.NextLines` _nextline)
        (set `self.DialogueIsFinished` (`KismetArrayLibrary.Array_IsEmpty` _nextline))
        (switch `int` _speakerid
          (:`0`
            (set `self.TextColor` (make `SlateColor` (struct :`R` 1.0 :`G` 1.0 :`B` 1.0 :`A` 1.0)))
            (bind _delay (`/Game/_Source/Dialogues/WB_DynamicSubtitles.ShowText` (`self.SubtitlesWidget`) (`self.CurrentPhrase`) 0.05 (`self.TextColor`)))
            (`KismetSystemLibrary.Delay` (+ _delay 1.0))
            (`KismetSystemLibrary.PrintString` "Finding Replies")
            (`self.FindReplies`)
            (`KismetSystemLibrary.PrintString` "Replies Found")
            (`self.ShowDialogueWidget` (`self.DialogueWidget`))
            (set `self.CurrentLIneName` (`|GetArrayItem` (`self.NextLines`) (`/Game/_Source/Dialogues/WB_Dialogue.ReplyID` (`self.DialogueWidget`))))
            (set `self.DialogueIsFinished` true))
          (:`1`
            (set `self.TextColor` (make `SlateColor` (struct :`R` 1.0 :`G` 0.666721 :`A` 1.0)))
            (bind _delay_2 (`/Game/_Source/Dialogues/WB_DynamicSubtitles.ShowText` (`self.SubtitlesWidget`) (`self.CurrentPhrase`) 0.05 (`self.TextColor`)))
            (`KismetSystemLibrary.Delay` (+ _delay_2 1.0))
            (set `self.CurrentLIneName` (`|GetArrayItem` (`self.NextLines`)))
            (set `self.DialogueIsFinished` true))))
      (:`RowNotFound`
        (break)))))

(fn `FindReplies`
  (`KismetArrayLibrary.Array_Clear` (`self.Replies`))
  (for _array_element (`self.NextLines`)
    (bind _returnvalue (`|GetDataTableRow` "/Game/_Source/Dialogues/CDT_Dialogues.CDT_Dialogues" _array_element)
      (:`then`
        (`KismetArrayLibrary.Array_Add` (`self.Replies`) (`.Text_5_05584FC849C5D8D42C4DC1B64A6CA068` (break `/Game/_Source/Dialogues/ST_DialogueLine` _returnvalue))))))
  (return))

(fn `RemoveSubtitle`)

(fn `ShowDialogueWidget`
  (params (Widget :type "/Game/_Source/Dialogues/WB_Dialogue Object Reference"))
  (`WidgetBlueprintLibrary.SetInputMode_UIOnlyEx` (`GameplayStatics.GetPlayerController` 0) null)
  (set `PlayerController.bShowMouseCursor` true (`GameplayStatics.GetPlayerController` 0))
  (`/Game/_Source/Dialogues/WB_Dialogue.Reply` (`self.DialogueWidget`) (`self.Replies`)))