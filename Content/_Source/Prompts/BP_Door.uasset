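; Interactable door Blueprint that cycles through closed, ajar and fully open on successive interactions.
; IsInteracting starts motion and a timer, during which Tick interpolates the door mesh's yaw toward the next state's angle.
; When the timer, timed by DoorSoundTime, fires, motion stops and the state advances.
; A facing dot product is meant to choose swing direction, but both branches set the same DoorSide, so it always swings one way.
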(event `self.ReceiveBeginPlay`
  (bind _asbp_first_person_character (cast `/Game/FirstPerson/Blueprints/BP_FirstPersonCharacter` (`GameplayStatics.GetPlayerCharacter` 0)))
  (set `self.CharacterRef` _asbp_first_person_character))

(event `self.ReceiveActorBeginOverlap`
  (params (OtherActor :type "Actor Object Reference")))

(event `self.ReceiveTick`
  (params (DeltaSeconds :type "Float (single-precision)"))
  (if (`self.InteractionDoor`)
    (`self.HandleDoor`)))

(event `Handle Interaction`
  (params (`Set Rotation` :type "Float (double-precision)"))
  ;[1 1 1] Door
  (`SceneComponent.K2_SetRelativeRotation` (`self.Door`) (`KismetMathLibrary.MakeRotator` 0.0 0.0 (`KismetMathLibrary.FInterpTo` (.yaw (`SceneComponent.RelativeRotation` (`self.Door`))) `Set Rotation` (`GameplayStatics.GetWorldDeltaSeconds`) (`self.Interp Speed`))) false false))

(event `IsInteracting`
  (params (Player :type "/Game/FirstPerson/Blueprints/BP_FirstPersonCharacter Object Reference"))
  ;[1 1 1] Door Interaction Math
  (if (> (`KismetMathLibrary.Dot_VectorVector` (`self.GetActorForwardVector` Player) (`SceneComponent.GetForwardVector` (`self.DoorLookLocation`))) 0.0)
    (set `self.DoorSide` 1.0)
    (else
      (set `self.DoorSide` 1.0)))
  (set `self.InteractionDoor` true)
  (`KismetSystemLibrary.K2_SetTimerDelegate` (delegate `CustomEvent`) (`self.Door Sound Time`)))

(event `CustomEvent`
  ;[1 1 1] Door Interaction Math
  (set `self.InteractionDoor` false)
  (switch `/Game/_Source/Prompts/E_DoorState` (`self.EDoorState`)
    (:`NewEnumerator0`
      (set `self.EDoorState` "NewEnumerator1"))
    (:`NewEnumerator1`
      (set `self.EDoorState` "NewEnumerator2"))
    (:`NewEnumerator2`
      (set `self.EDoorState` "NewEnumerator0"))))

(event `HandleDoor`
  ;[1 1 1] Handle Door
  (switch `/Game/_Source/Prompts/E_DoorState` (`self.EDoorState`)
    (:`NewEnumerator0`
      (`self.Handle Interaction` (* (`self.DoorSide`) 15.0)))
    (:`NewEnumerator1`
      (`self.Handle Interaction` (* (`self.DoorSide`) (`self.OpenAngle`))))
    (:`NewEnumerator2`
      (`self.Handle Interaction` 0.0))))

(fn `UserConstructionScript`)